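; Wolf AI character in Young, Adult and Alpha variants that set health, stamina, meat drop and XP reward.
; It roams to random reachable points while Tick drains stamina, slowing it when tired and triggering a Rest loop that recovers stamina before roaming resumes.
; Damage spawns an indicator and plays a hit montage; death spawns meat and awards XP through the game mode.
; A widget healthbar tracks health and animates in and out through show/hide events.
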(event `HideHealthbar`
  (set `self.PlayerLooking` false)
  (`KismetSystemLibrary.Delay` 1.0)
  (if (not (`self.PlayerLooking`))
    (bind _aswolf_healthbar_ui (cast `/Game/UI/Wolf_Healthbar_UI` (`WidgetComponent.GetUserWidgetObject` (`self.Healthbar`))))
    (`UserWidget.PlayAnimation` _aswolf_healthbar_ui (`/Game/UI/Wolf_Healthbar_UI.Intro` _aswolf_healthbar_ui) 0.0 1 "Forward" 1.0 false)
    (`KismetSystemLibrary.Delay` 0.5)
    (if (not (`self.PlayerLooking`))
      (`SceneComponent.SetVisibility` (`self.Healthbar`) false false))))

(event `VisibleHealthbar`
  (bind _healthbar (`self.Healthbar`))
  (if (not (`self.PlayerLooking`))
    (set `self.PlayerLooking` true)
    (`SceneComponent.SetVisibility` _healthbar true false)
    (bind _aswolf_healthbar_ui (cast `/Game/UI/Wolf_Healthbar_UI` (`WidgetComponent.GetUserWidgetObject` _healthbar)))
    (`UserWidget.PlayAnimation` _aswolf_healthbar_ui (`/Game/UI/Wolf_Healthbar_UI.Intro` _aswolf_healthbar_ui) 0.0 1 "Reverse" 1.0 false)))

(event `self.ReceiveBeginPlay`
  (`|ExecutionSequence`
    (:`then_0`
      (set `self.Health` (`self.Max_Health`))
      (`self.Roam`))
    (:`then_1`
      (switch `/Game/Blueprints/Enums/Animal_Type_Enum` (`self.AnimalType`)
        (:`NewEnumerator0`
          (bind _output_get (set `self.Max_Health` 100.0))
          (set `self.Health` _output_get)
          (set `self.Stamina` 150.0))
        (:`NewEnumerator1`
          (bind _output_get_2 (set `self.Max_Health` 200.0))
          (set `self.Health` _output_get_2)
          (set `self.Stamina` 300.0))
        (:`NewEnumerator2`
          (bind _output_get_3 (set `self.Max_Health` 400.0))
          (set `self.Health` _output_get_3)
          (set `self.Stamina` 500.0))))
    (:`then_2`
      (bind _aswolf_healthbar_ui (cast `/Game/UI/Wolf_Healthbar_UI` (`WidgetComponent.GetWidget` (`self.Healthbar`))))
      (switch `/Game/Blueprints/Enums/Animal_Type_Enum` (`self.AnimalType`)
        (:`NewEnumerator0`
          (`/Game/UI/Wolf_Healthbar_UI.SetStats` _aswolf_healthbar_ui "Young Wolf"))
        (:`NewEnumerator1`
          (`/Game/UI/Wolf_Healthbar_UI.SetStats` _aswolf_healthbar_ui "Adult Wolf"))
        (:`NewEnumerator2`
          (`/Game/UI/Wolf_Healthbar_UI.SetStats` _aswolf_healthbar_ui "Alpha Wolf"))))
    (:`then_3`
      (bind _asbp_game_game_mode (cast `/Game/InventoryKit/Framework/BP_GameGameMode` (`GameplayStatics.GetGameMode`)))
      (set `self.As BP Game Game Mode` _asbp_game_game_mode))))

(event `Roam`
  (if (not (`self.Resting`))
    (`|AIMoveTo` self (`NavigationSystemV1.K2_GetRandomReachablePointInRadius` (`self.K2_GetActorLocation`) 2000.0 null null) null
      (:`OnSuccess`
        (`KismetSystemLibrary.Delay` (`KismetMathLibrary.RandomFloatInRange` 2.0 5.0))
        (`self.Roam`)))))

(event `self.ReceiveTick`
  (params (DeltaSeconds :type "Float (single-precision)"))
  (bind _drain (`self.Drain`))
  (`|ExecutionSequence`
    (:`then_0`
      (if (not (`self.Resting`))
        (`KismetSystemLibrary.Delay` 1.0)
        (`self.DrainStamina`)
        (set `self.Stamina` (- (`self.Stamina`) (`KismetMathLibrary.RandomFloatInRange` (/ _drain 2.0) _drain)))
        (bind _exausted (`self.CheckStamina`))
        (if _exausted
          (`self.Rest`))))
    (:`then_1`
      (`self.UpdateHealthbar`))))

(event `self.ReceiveAnyDamage`
  (params (Damage :type "Float (single-precision)") (DamageType :type "DamageType Object Reference") (InstigatedBy :type "Controller Object Reference") (DamageCauser :type "Actor Object Reference"))
  (`|SpawnActorFromClass` "/Game/Blueprints/DamabeIndicator_BP.DamabeIndicator_BP_C" (`self.GetTransform`) "Undefined" "MultiplyWithRoot" null Damage null)
  (bind _output_get (set `self.Health` (`KismetMathLibrary.FClamp` (- (`self.Health`) Damage) 0.0 (`self.Max_Health`))))
  (if (== _output_get 0.0)
    (`self.Death`)
    (else
      (`self.PlayAnimMontage` "/Game/AnimalVarietyPack/Wolf/Animations/ANIM_Wolf_GetHitFront_Montage.ANIM_Wolf_GetHitFront_Montage"))))

(event `Death`
  (bind _animaltype (`self.AnimalType`))
  (`/Engine/EditorBlueprintResources/StandardMacros.DoOnce` false
    (:`Completed`
      (set `self.Resting` true)
      (set `CharacterMovementComponent.MaxWalkSpeed` 0.0 (`self.CharacterMovement`))
      (`SkeletalMeshComponent.PlayAnimation` (`self.Mesh`) "/Game/AnimalVarietyPack/Wolf/Animations/ANIM_Wolf_Death.ANIM_Wolf_Death" false)
      (`self.SpawnMeat` (select `/Game/Blueprints/Enums/Animal_Type_Enum` _animaltype :`NewEnumerator0` 1 :`NewEnumerator1` 2 :`NewEnumerator2` 4))
      (`/Game/InventoryKit/Framework/BP_GameGameMode.AddXP` (`self.As BP Game Game Mode`) (select `/Game/Blueprints/Enums/Animal_Type_Enum` _animaltype :`NewEnumerator0` 50.0 :`NewEnumerator1` 120.0 :`NewEnumerator2` 200.0)))))

(fn `CheckStamina`
  (returns (Exausted :type Boolean))
  (bind _stamina (`self.Stamina`))
  (if (and (<= _stamina 30.0) (> _stamina 5.0))
    (set `CharacterMovementComponent.MaxWalkSpeed` 150.0 (`self.CharacterMovement`))
    (set `self.Tired` true)
    (return false)
    (elif (<= (`self.Stamina`) 4.0)
      (return true)
      (else
        (return false)))))

(fn `DrainStamina`
  (bind _maxwalkspeed (`CharacterMovementComponent.MaxWalkSpeed` (`self.CharacterMovement`)))
  (if (== _maxwalkspeed 600.0)
    (set `self.Drain` 10.0)
    (elif (== _maxwalkspeed 0.0)
      (set `self.Drain` 5.0)
      (else
        (set `self.Drain` 5.0))))
  (return))

(fn `Sleep`)

(fn `SpawnMeat`
  (params (MeatToSpawn :type Integer))
  (bind _randomlocation (`NavigationSystemV1.K2_GetRandomReachablePointInRadius` (`self.K2_GetActorLocation`) 100.0 null null))
  (for _ (range (+ MeatToSpawn 1))
    (`|SpawnActorFromClass` "/Game/Blueprints/Items/Meat_Item.Meat_Item_C" (`KismetMathLibrary.MakeTransform` (`KismetMathLibrary.MakeVector` (.x _randomlocation) (.y _randomlocation) (- (.z _randomlocation) 90.0)) (`KismetMathLibrary.MakeRotator` 0.0 0.0 (`KismetMathLibrary.RandomFloatInRange` 0.0 360.0))) "Undefined" "MultiplyWithRoot" null null))
  (return))

(fn `UpdateHealthbar`
  (bind _aswolf_healthbar_ui (cast `/Game/UI/Wolf_Healthbar_UI` (`WidgetComponent.GetUserWidgetObject` (`self.Healthbar`))))
  (set `/Game/UI/Wolf_Healthbar_UI.Health` (`self.Health`) _aswolf_healthbar_ui)
  (set `/Game/UI/Wolf_Healthbar_UI.MaxHealth` (`self.Max_Health`) _aswolf_healthbar_ui))

(fn `UserConstructionScript`)