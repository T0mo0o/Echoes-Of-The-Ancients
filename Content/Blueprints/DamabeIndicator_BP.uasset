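; Floating damage number actor that displays a damage amount through its Widget component, then removes itself.
; On BeginPlay it copies DmgAmt into the Dmage_Indicator_UI widget and stops if that cast fails.
; The PlayAnim timeline then lerps the actor from its spawn location to a fixed world-space offset, upward and slightly sideways, and destroys it when finished.
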(event `self.ReceiveBeginPlay`
  (bind _asdmage_indicator_ui (cast `/Game/UI/Dmage_Indicator_UI` (`WidgetComponent.GetWidget` (`self.Widget`))))
  (set `/Game/UI/Dmage_Indicator_UI.DmgAmt` (`self.Dmg Amt`) _asdmage_indicator_ui)
  (bind _output_get (set `self.StartLocation` (`self.K2_GetActorLocation`)))
  (set `self.EndLocation` (+ _output_get (-25.0 -25.0 50.0)))
  (bind (_direction _newtrack_0) (`Timeline|PlayAnim`)
    (:`Update`
      (`self.K2_SetActorLocation` (`KismetMathLibrary.VLerp` (`self.StartLocation`) (`self.EndLocation`) _newtrack_0)))
    (:`Finished`
      (`self.K2_DestroyActor`))))

(fn `UserConstructionScript`)