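; Meat pickup item that shows its icon on a world widget and pops a collected message on overlap.
; BeginPlay copies the ItemInfo icon into the widget's image.
; Sphere overlap by any Interact_BP actor creates the message widget, then switches on the game mode's possessed-character enum with nothing connected.
; The AddToInventory and DestroyActor nodes are unreachable, so the item is neither stored nor removed here.
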(event `self.ReceiveBeginPlay`
  (bind (_iteminfo_name _iteminfo_icon) (break `/Game/Blueprints/Structs/ItemInfo_Struct` (`self.ItemInfo`)))
  (bind _asitem_world_icon_ui (cast `/Game/UI/Inventory/Item_World_Icon_UI` (`WidgetComponent.GetWidget` (`self.Widget`))))
  (`Image.SetBrushFromTexture` (`/Game/UI/Inventory/Item_World_Icon_UI.Image_34` _asitem_world_icon_ui) _iteminfo_icon false))

(event `self.Sphere.OnComponentBeginOverlap`
  (params (OverlappedComponent :type "PrimitiveComponent Object Reference") (OtherActor :type "Actor Object Reference") (OtherComp :type "PrimitiveComponent Object Reference") (OtherBodyIndex :type Integer) (bFromSweep :type Boolean) (SweepResult :type "HitResult Structure (by ref)"))
  (bind _iteminfo_name (break `/Game/Blueprints/Structs/ItemInfo_Struct` (`self.ItemInfo`)))
  (if (`KismetSystemLibrary.DoesImplementInterface` OtherActor "/Game/Blueprints/Interact_BP.Interact_BP_C")
    (bind _returnvalue (`|CreateWidget` "/Game/UI/Item_Collected_Message_UI.Item_Collected_Message_UI_C" null 1 _iteminfo_name))
    (`UserWidget.AddToViewport` _returnvalue 0)
    (bind _asbp_third_person_game_mode (cast `/Game/ThirdPerson/Blueprints/BP_ThirdPersonGameMode` (`GameplayStatics.GetGameMode`)))
    (switch `/Game/Blueprints/Enums/Character_Possesed_Enum` (`/Game/ThirdPerson/Blueprints/BP_ThirdPersonGameMode.CharacterPossesedEnum` _asbp_third_person_game_mode))))

(fn `UserConstructionScript`)