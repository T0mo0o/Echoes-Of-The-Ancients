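; Sword pickup actor that adds its item to the possessed character's inventory hotbar when touched.
; A sphere overlap with any actor implementing Interact_BP shows a collected-message widget with the item's name.
; It then reads the possessed-character enum from BP_ThirdPersonGameMode, passes ItemInfo to the Chimalli or Colel hotbar through the player UI reference, and destroys itself.
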(event `self.Sphere.OnComponentBeginOverlap`
  (params (OverlappedComponent :type "PrimitiveComponent Object Reference") (OtherActor :type "Actor Object Reference") (OtherComp :type "PrimitiveComponent Object Reference") (OtherBodyIndex :type Integer) (bFromSweep :type Boolean) (SweepResult :type "HitResult Structure (by ref)"))
  (bind _iteminfo_name (break `/Game/Blueprints/Structs/ItemInfo_Struct` (`self.ItemInfo`)))
  (bind _iteminfo (`self.ItemInfo`))
  (if (`KismetSystemLibrary.DoesImplementInterface` OtherActor "/Game/Blueprints/Interact_BP.Interact_BP_C")
    (bind _returnvalue (`|CreateWidget` "/Game/UI/Item_Collected_Message_UI.Item_Collected_Message_UI_C" null 1 _iteminfo_name))
    (`UserWidget.AddToViewport` _returnvalue 0)
    (bind _asbp_third_person_game_mode (cast `/Game/ThirdPerson/Blueprints/BP_ThirdPersonGameMode` (`GameplayStatics.GetGameMode`)))
    (switch `/Game/Blueprints/Enums/Character_Possesed_Enum` (`/Game/ThirdPerson/Blueprints/BP_ThirdPersonGameMode.CharacterPossesedEnum` _asbp_third_person_game_mode)
      (:`NewEnumerator0`
        (bind _player_ui_ref (`/Game/ThirdPerson/Blueprints/BP_ThirdPersonGameMode.Player_UI_Ref` _asbp_third_person_game_mode))
        (`/Game/UI/Inventory/Chimalli_Inventory_Hotbar_UI.AddToInventory` (`/Game/UI/Player_UI.Chimalli_Inventory_Hotbar_UI` _player_ui_ref) _iteminfo))
      (:`NewEnumerator1`
        (`/Game/UI/Inventory/Colel_Inventory_Hotbar_UI.AddToInventory` (`/Game/UI/Player_UI.Colel_Inventory_Hotbar_UI` _player_ui_ref) _iteminfo)))
    (`self.K2_DestroyActor`)))

(fn `UserConstructionScript`)